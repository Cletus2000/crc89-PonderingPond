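; BP_Spawn is a spawner actor that populates the area around itself with BP_Fish actors when play begins.
; BeginPlay runs a fixed-count loop, spawning each fish at the actor's location plus a random X and Y offset scaled by Radius.
; The Z term uses a constant that evaluates to zero, so fish spread over a flat square at the spawner's height rather than a volume.
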(event EventBeginPlay
  (bind _radius (Variables|Default|GetRadius))
  (for _index (range 0 10)
    (Game|SpawnActorfromClass "/Game/BP_Fish.BP_Fish_C" (Math|Transform|MakeTransform (+ (Transformation|GetActorLocation) (Math|Vector|MakeVector (* (* (- (Math|Random|RandomFloat) 0.5) 2.0) _radius) (* (* (- (Math|Random|RandomFloat) 0.5) 2.0) _radius) (* (* (- 0.5 0.5) 2.0) _radius))) "0, 0, 0" "1.000000,1.000000,1.000000") "Undefined" "MultiplyWithRoot" 0 0)))

(fn ConstructionScript)